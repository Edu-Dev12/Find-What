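; BP_DeliveryZone is a drop-off zone that accepts the item assigned to the first-person player controller.
; Shortly after BeginPlay it copies the controller's OwnItem mesh onto a miniature preview, which spins every tick.
; When an Item overlaps the cylinder and its mesh matches the controller's current OwnItem, the zone calls ObjectFound on the controller and destroys the item.
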(event OnComponentBeginOverlap(Cylinder)
  (params (OverlappedComponent :type Primitive%20Component%20Object%20Reference) (OtherActor :type Actor%20Object%20Reference) (OtherComp :type Primitive%20Component%20Object%20Reference) (OtherBodyIndex :type Integer) (bFromSweep :type Boolean) (SweepResult :type Hit%20Result%20Structure%20%28by%20ref%29))
  (bind _asitem (Utilities|Casting|CastToItem OtherActor))
  (bind _asbp_first_person_player_controller (Utilities|Casting|CastToBP_FirstPersonPlayerController (Game|GetPlayerController 0)))
  (if (== (Variables|/Game/FirstPerson/Blueprints/BP_FirstPersonPlayerController.BP_FirstPersonPlayerController_C|GetOwnItem _asbp_first_person_player_controller) (Variables|/Script/Engine.StaticMeshComponent|GetStaticMesh (Variables|/Game/Scripts/Item.Item_C|GetItem _asitem)))
    (Default|ObjectFound _asbp_first_person_player_controller)
    (Actor|DestroyActor _asitem)))

(event EventBeginPlay
  (Utilities|FlowControl|Delay 0.5)
  (bind _asbp_first_person_player_controller (Utilities|Casting|CastToBP_FirstPersonPlayerController (Game|GetPlayerController 0)))
  (Components|StaticMesh|SetStaticMesh (Variables|Default|GetItemMiniatura) (Variables|/Game/FirstPerson/Blueprints/BP_FirstPersonPlayerController.BP_FirstPersonPlayerController_C|GetOwnItem _asbp_first_person_player_controller)))

(event EventTick
  (params (DeltaSeconds :type Float%20%28single-precision%29))
  (Transformation|AddWorldRotation (Variables|Default|GetItemMiniatura) (Math|Rotator|MakeRotator 0.0 0.0 1.0) false false))

(fn ConstructionScript)